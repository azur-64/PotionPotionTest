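; BP_PlayerCharacter is the player character, driven by Enhanced Input with smoothed movement and turning.
; BeginPlay adds the player mapping context and sets the CineCamera's depth of field, using the spring arm length as focal distance.
; IA_Move input maps to world XY, interpolating both actor rotation and a stored movement vector toward that direction before feeding it to AddMovementInput.
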(event `self.ReceiveBeginPlay`
  (bind _cinecamera (`self.CineCamera`))
  (`EnhancedInputSubsystemInterface.AddMappingContext` (pcsubsystem `EnhancedInputLocalPlayerSubsystem` (`GameplayStatics.GetPlayerController` 0)) "/Game/PotionPotionDemo/Input/IMC_PlayerCharacter.IMC_PlayerCharacter" 0 (struct))
  (bind _structout (setmembers `PostProcessSettings` :`StructRef` (`CameraComponent.PostProcessSettings` _cinecamera) :`DepthOfFieldFstop` 0.5 :`DepthOfFieldSensorWidth` 150.0 :`DepthOfFieldFocalDistance` (`SpringArmComponent.TargetArmLength` (`self.SpringArm`))))
  (set `CameraComponent.PostProcessSettings` _structout _cinecamera))

(event `EnhancedInput|/Game/PotionPotionDemo/Input/IA_Move`
  (params (ActionValue :type "Vector2D Structure") (ElapsedSeconds :type "Float (double-precision)") (TriggeredSeconds :type "Float (double-precision)") (InputAction :type "InputAction Object Reference" :default "/Game/PotionPotionDemo/Input/IA_Move.IA_Move"))
  (bind _returnvalue (`GameplayStatics.GetWorldDeltaSeconds`))
  (bind _returnvalue_2 (`KismetMathLibrary.Normal` (`KismetMathLibrary.MakeVector` ActionValue_X ActionValue_Y)))
  (:`Triggered`
    (`self.K2_SetActorRotation` (`KismetMathLibrary.RInterpTo` (`self.K2_GetActorRotation`) (`KismetMathLibrary.MakeRotFromX` _returnvalue_2) _returnvalue 4.0))
    (bind _output_get (set `self.MovementVector` (`KismetMathLibrary.VInterpTo` (`self.MovementVector`) (* _returnvalue_2 1.5) _returnvalue 4.0)))
    (`self.AddMovementInput` _output_get)))

(fn `UserConstructionScript`)